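; BP_Garden is a garden plot actor that grows a vegetable through None, Growing and Ready for Harvest states.
; Planting enables Tick, which increments a counter per tick and prints the remaining count as minutes:seconds until GrowingDuration is reached.
; Readiness shows the Vegetable and stops Tick, while harvesting hides it and resets the plot.
; SaveGarden and LoadGarden pass state, progress and tick status through an SGardenInformation struct.
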(event `self.ReceiveTick`
  (params (DeltaSeconds :type "Float (single-precision)"))
  (`self.D_PrintGrowingProgress`)
  (bind _result (`/Engine/EditorBlueprintResources/StandardMacros.IncrementInt` (`self.CurrentGrowingDuration`))
    (:`  `
      (if (>= _result (`self.GrowingDuration`))
        (`self.TriggerVegetableReadyForHarvest`)))))

(fn `CanPlantVegetable`
  (returns (CanPlant :type Boolean))
  (switch `/Game/_Enums/E_VegetableStatus` (`self.eVegetableStatus`)
    (:`NewEnumerator0`
      (return true))
    (:`NewEnumerator1`
      _)
    (:`NewEnumerator2`
      _))
  (`KismetSystemLibrary.PrintString` "Can't plant vegetable here !")
  (return false))

(fn `D_PrintGrowingProgress`
  (bind _returnvalue (- (`self.GrowingDuration`) (+ (`self.CurrentGrowingDuration`) 1)))
  (bind _returnvalue_2 (mod _returnvalue 60))
  (`KismetSystemLibrary.PrintString` (`KismetStringLibrary.Concat_StrStr` (`KismetStringLibrary.Conv_IntToString` (/ _returnvalue 60)) ":" (`KismetStringLibrary.Conv_IntToString` (/ _returnvalue_2 10)) (`KismetStringLibrary.Conv_IntToString` (mod _returnvalue_2 10))) true false (struct :`G` 0.66 :`B` 1.0 :`A` 1.0) 1.0))

(fn `HarvestVegetable`
  (returns (Harvested :type Boolean))
  (switch `/Game/_Enums/E_VegetableStatus` (`self.eVegetableStatus`)
    (:`NewEnumerator0`
      _)
    (:`NewEnumerator1`
      _)
    (:`NewEnumerator2`
      (`SceneComponent.SetVisibility` (`self.Vegetable`) false false)
      (set `self.CurrentGrowingDuration` 0)
      (`self.SetActorTickEnabled` false)
      (set `self.eVegetableStatus` "NewEnumerator0")
      (return true)))
  (`KismetSystemLibrary.PrintString` "Can't harvest now")
  (return false))

(fn `LoadGarden`
  (params (GardenInformation :type "/Game/_Enums/S_GardenInformation Structure"))
  (bind (_vegetablename _growingduration _currentgrowingduration _bisvegetablegrowing _evegetablestatus _bisactortickenabled) (break `/Game/_Enums/S_GardenInformation` GardenInformation))
  (set `self.VegetableName` _vegetablename)
  (set `self.GrowingDuration` _growingduration)
  (set `self.CurrentGrowingDuration` _currentgrowingduration)
  (bind _output_get (set `self.eVegetableStatus` _evegetablestatus))
  (`self.SetActorTickEnabled` _bisactortickenabled)
  (`SceneComponent.SetVisibility` (`self.Vegetable`) (`|EnumEquality` _output_get "NewEnumerator2") false))

(fn `PlantVegetable`
  (switch `/Game/_Enums/E_VegetableStatus` (`self.eVegetableStatus`)
    (:`NewEnumerator0`
      (set `self.eVegetableStatus` "NewEnumerator1")
      (`self.SetActorTickEnabled` true))
    (:`NewEnumerator1`
      (`KismetSystemLibrary.PrintString` "Can't plant vegetable here !" :!label _label))
    (:`NewEnumerator2`
      (goto _label)))
  (return))

(fn `SaveGarden`
  (returns (GardenData :type "/Game/_Enums/S_GardenInformation Structure"))
  (return (make `/Game/_Enums/S_GardenInformation` (`self.VegetableName`) (`self.GrowingDuration`) (`self.CurrentGrowingDuration`) false (`self.eVegetableStatus`) (`self.IsActorTickEnabled`))))

(fn `TriggerVegetableReadyForHarvest`
  (`SceneComponent.SetVisibility` (`self.Vegetable`) true false)
  (set `self.eVegetableStatus` "NewEnumerator2")
  (`self.SetActorTickEnabled` false))

(fn `UserConstructionScript`)