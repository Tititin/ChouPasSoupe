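; Inventory Blueprint that tracks how many of each vegetable is held, using a name-to-count map.
; AddVegetable and TakeVegetable change the counts and push them to the InventoryUI widget, with Take returning false when none remain.
; ToggleInventory shows or hides the widget, refreshing all slots before showing it.
; InitInventoryUI builds slots from the map, while BeginPlay is empty and the EventGraph's UI setup is disconnected.
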(event `self.ReceiveBeginPlay`)

(fn `AddVegetable`
  (params (VegetableName :type Name))
  (bind _vegetables (`self.Vegetables`))
  (bind (_value _returnvalue) (`BlueprintMapLibrary.Map_Find` (`self.Vegetables`) VegetableName))
  (if _returnvalue
    (bind _result (`/Engine/EditorBlueprintResources/StandardMacros.IncrementInt` _value)
      (:`  `
        (`BlueprintMapLibrary.Map_Add` _vegetables VegetableName _result)))
    (else
      (`BlueprintMapLibrary.Map_Add` _vegetables VegetableName 1)))
  ;[1 1 0] DEBUG
  (`KismetSystemLibrary.PrintString` (`KismetStringLibrary.Concat_StrStr` "Added : " (`KismetStringLibrary.Conv_NameToString` VegetableName)))
  (`self.UpdateInventorySlot` VegetableName _result)
  (return))

(fn `D_PrintInventory`
  (bind _vegetables (`self.Vegetables`))
  (bind _keys (`BlueprintMapLibrary.Map_Keys` _vegetables))
  (for _array_element _keys
    (`KismetSystemLibrary.PrintString` (`KismetStringLibrary.Concat_StrStr` (`KismetStringLibrary.Conv_NameToString` _array_element) " : " (`KismetStringLibrary.Conv_IntToString` (`BlueprintMapLibrary.Map_Find` _vegetables _array_element))))
    (return)))

(fn `InitInventoryUI`
  (bind _vegetables (`self.Vegetables`))
  (bind _keys (`BlueprintMapLibrary.Map_Keys` _vegetables))
  (for _array_element _keys
    (`/Game/_2D/W_Inventory.AddInventorySlot` (`self.InventoryUI`) _array_element (`BlueprintMapLibrary.Map_Find` _vegetables _array_element))))

(fn `TakeVegetable`
  (params (VegetableName :type Name))
  (returns (bIsTaken :type Boolean))
  (bind (_value _returnvalue) (`BlueprintMapLibrary.Map_Find` (`self.Vegetables`) VegetableName))
  (if (and _returnvalue (> _value 0))
    (bind _result (`/Engine/EditorBlueprintResources/StandardMacros.DecrementInt` _value)
      (:`  `
        ;[1 1 0] DEBUG
        (`BlueprintMapLibrary.Map_Add` (`self.Vegetables`) VegetableName _result)
        (`self.UpdateInventorySlot` VegetableName _result)
        (return true)))
    (else
      (`KismetSystemLibrary.PrintString` "No more of this vegetable in the inventory !")
      (return false))))

(fn `ToggleInventory`
  (bind _inventoryui (`self.InventoryUI`))
  (switch `ESlateVisibility` (`Widget.GetVisibility` _inventoryui)
    (:`Visible`
      (`Widget.SetVisibility` _inventoryui "Hidden"))
    (:`Hidden`
      (`self.UpdateInventory`)
      (`Widget.SetVisibility` _inventoryui "Visible"))))

(fn `UpdateInventory`
  (bind _vegetables (`self.Vegetables`))
  (bind _keys (`BlueprintMapLibrary.Map_Keys` _vegetables))
  (for _array_element _keys
    (`self.UpdateInventorySlot` _array_element (`BlueprintMapLibrary.Map_Find` _vegetables _array_element))))

(fn `UpdateInventorySlot`
  (params (ItemName :type Name) (Amount :type Integer))
  (`/Game/_2D/W_Inventory.UpdateInventorySlot` (`self.InventoryUI`) ItemName Amount)
  (return))