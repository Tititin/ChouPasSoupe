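; Save game object that stores and restores the player's vegetable inventory and the state of the gardens.
; Inventory save and load copy the Vegetables map key by key, clearing the target only on load.
; Each garden serializes itself through SaveGarden and LoadGarden into GardensInformation, matched back by array index, so garden order must stay consistent.
; An older field-by-field garden restore remains as unconnected nodes.
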(fn `LoadGardens`
  (params (Gardens :type "Array of /Game/_BP/BP_Garden Object Reference (by ref)"))
  (for (_array_element _array_index) Gardens
    (`/Game/_BP/BP_Garden.LoadGarden` _array_element (`|GetArrayItem` (`self.GardensInformation`) _array_index)))
  (return))

(fn `LoadInventory`
  (params (UserInventory :type "/Game/_BP/BP_Inventory Object Reference (by ref)"))
  (bind _vegetables (`/Game/_BP/BP_Inventory.Vegetables` UserInventory))
  (bind _vegetables_2 (`self.Vegetables`))
  (`BlueprintMapLibrary.Map_Clear` _vegetables)
  (bind _keys (`BlueprintMapLibrary.Map_Keys` _vegetables_2))
  (for _array_element _keys
    (`BlueprintMapLibrary.Map_Add` _vegetables _array_element (`BlueprintMapLibrary.Map_Find` _vegetables_2 _array_element)))
  (return))

(fn `SaveGardens`
  (params (Gardens :type "Array of /Game/_BP/BP_Garden Object Reference"))
  (`KismetArrayLibrary.Array_Clear` (`self.GardensInformation`))
  (for _array_element Gardens
    (bind _gardendata (`/Game/_BP/BP_Garden.SaveGarden` _array_element))
    (`KismetArrayLibrary.Array_Add` (`self.GardensInformation`) _gardendata))
  (return))

(fn `SaveInventory`
  (params (UserInventory :type "/Game/_BP/BP_Inventory Object Reference"))
  (bind _vegetables (`/Game/_BP/BP_Inventory.Vegetables` UserInventory))
  (bind _keys (`BlueprintMapLibrary.Map_Keys` _vegetables))
  (for _array_element _keys
    (`BlueprintMapLibrary.Map_Add` (`self.Vegetables`) _array_element (`BlueprintMapLibrary.Map_Find` _vegetables _array_element)))
  (return))